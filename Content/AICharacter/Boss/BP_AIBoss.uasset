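; Boss AI character that runs a behavior tree and can catch the player.
; On BeginPlay it has its BP_AIController run BT_Main, while exposing walk speed control and getters for jump-attack and caught-player state.
; A hit on CatchPlayerCollision by an FPSMannequin sets the caught flag and prints debug names.
; Events play attack and victory montages, with the attack routed through an event pair labeled server and multicast.
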(event EventBeginPlay
  (bind _asbp_aicontroller (Utilities|Casting|CastToBP_AIController (Pawn|GetController)))
  (bind _output_get (Variables|Default|SetOwnController _asbp_aicontroller))
  (AI|RunBehaviorTree _output_get "/Game/AICharacter/Boss/BT_Main.BT_Main"))

(event EventSetWalkSpeed
  (params (speed :type Float%20%28single-precision%29))
  (Variables|/Script/Engine.CharacterMovementComponent|SetMaxWalkSpeed (Variables|Character|GetCharacterMovement) speed))

(event OnComponentHit(CatchPlayerCollision)
  (params (HitComponent :type Primitive%20Component%20Object%20Reference) (OtherActor :type Actor%20Object%20Reference) (OtherComp :type Primitive%20Component%20Object%20Reference) (NormalImpulse :type Vector :default "0, 0, 0") (Hit :type Hit%20Result%20Structure%20%28by%20ref%29))
  (bind _asfpsmannequin (Utilities|Casting|CastToFPSMannequin OtherActor))
  (Variables|Default|SetbPlayerIsCatched true)
  (Development|PrintString (Utilities|GetDisplayName _asfpsmannequin))
  (Development|PrintString (Utilities|GetDisplayName (Game|GetGameMode))))

(event Custom|MC_PlayAttackAnim
  ;[1 0 0] Attack Anim Play Server & MultiCast
  (Animation|PlayAnimMontage "/Game/AICharacter/BOOS/AM_Attack.AM_Attack" 3.0 "None")
  (Utilities|FlowControl|Delay 4.0))

(event EventPlayVictoryAnim
  (Animation|PlayAnimMontage "/Game/AICharacter/BOOS/Anim/Attack/AM_Victory.AM_Victory" 0.8 "None"))

(event EventPlayAttackAnim
  ;[1 0 0] Attack Anim Play Server & MultiCast
  (CallFunction|MCPlayAttackAnim))

(fn ConstructionScript
  (Variables|/Script/Engine.CharacterMovementComponent|SetMaxWalkSpeed (Variables|Character|GetCharacterMovement) 2.5e+02))

(fn GetEnableJumpAttack
  (return (Variables|Default|GetbAttackJump)))

(fn PlayerIsCatched
  (return (Variables|Default|GetbPlayerIsCatched)))