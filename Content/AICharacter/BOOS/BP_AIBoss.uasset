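; AI boss character that starts a behavior tree through its controller and can jump or climb ledges while the player is seen.
; Each tick then, two sphere traces measure the ledge ahead and select a jump or climb, played as a montage with MoveComponentTo onto the hit point.
; An overlap volume briefly flags the player as caught.
; Events and getters expose sight, suspicion and hit state, plus attack, victory and directional turn montages.
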(event Custom|JumpEvent
  ;[1 0 0] Jump events
  (Utilities|FlowControl|DoOnce false :!label _label
    (:Completed
      (Animation|PlayAnimMontage "/Game/AICharacter/BOOS/Anim/Jump/AM_Jump_Boss.AM_Jump_Boss" 1.0 "JumpUp")
      (Utilities|FlowControl|Delay 1.2)
      (Components|MoveComponentTo (Variables|Default|GetCapsuleComponent) (+ (.impactpoint (Variables|Default|GetHitLedgeUp)) (Math|Vector|MakeVector 0.0 0.0 (Components|Capsule|GetScaledCapsuleHalfHeight (Variables|Default|GetCapsuleComponent)))) (Transformation|GetActorRotation) false false 0.4 false)
      (Variables|Default|SetBoss_JumpState "NewEnumerator1")
      (Utilities|FlowControl|Delay 1.2)
      (goto _label Reset))))

(event Custom|HandAndClimb
  (bind _charactermovement (Variables|Character|GetCharacterMovement))
  ;[1 0 0] Jump events
  (Utilities|FlowControl|DoOnce false :!label _label
    (:Completed
      (Animation|PlayAnimMontage "/Game/AICharacter/BOOS/Anim/Climb/AM_Boss_Climb.AM_Boss_Climb" 1.0 "Jump_Climb")
      (Pawn|Components|CharacterMovement|SetMovementMode _charactermovement "MOVE_Flying" 0)
      (Components|MoveComponentTo (Variables|Default|GetCapsuleComponent) (- (.impactpoint (Variables|Default|GetHitLedgeUp)) (Math|Vector|MakeVector 0.0 0.0 (+ (Components|Capsule|GetScaledCapsuleHalfHeight (Variables|Default|GetCapsuleComponent)) 5e+01))) (Transformation|GetActorRotation) false false 0.4 false)
      (Utilities|FlowControl|Delay 1.5)
      (Pawn|Components|CharacterMovement|SetMovementMode _charactermovement "MOVE_Walking" 0)
      (Variables|Default|SetBoss_JumpState "NewEnumerator1")
      (Utilities|FlowControl|Delay 2.0)
      (goto _label Reset))))

(event Custom|SetJumpPermision
  (params (Enable :type Boolean))
  ;[1 1 1] No More Use this
  (Variables|Default|SetbJumpOn Enable))

(event EventBeginPlay
  (bind _asabp_boss (Utilities|Casting|CastToABP_BOSS (Components|SkeletalMesh|GetAnimInstance (Variables|Character|GetMesh))))
  (Variables|Default|SetAnimInstance _asabp_boss)
  (bind _asbp_aicontroller (Utilities|Casting|CastToBP_AIController (Pawn|GetController)))
  (bind _output_get (Variables|Default|SetOwnController _asbp_aicontroller))
  (AI|RunBehaviorTree _output_get (Variables|Default|GetBT_Main)))

(event EventOnLanded
  (params (Hit :type Hit%20Result%20Structure%20%28by%20ref%29))
  (bind _charactermovement (Variables|Character|GetCharacterMovement))
  ;[1 0 0] Jump events
  (Animation|PlayAnimMontage "/Game/AICharacter/BOOS/Anim/Jump/AM_Jump_Boss.AM_Jump_Boss" 1.2 "JumpDown")
  (Pawn|Components|CharacterMovement|SetMovementMode _charactermovement "MOVE_None" 0)
  (Utilities|FlowControl|Delay 1.0)
  (Pawn|Components|CharacterMovement|SetMovementMode _charactermovement "MOVE_Walking" 0))

(event EventTick
  (params (DeltaSeconds :type Float%20%28single-precision%29))
  (if (Variables|Default|GetPlayerIsSeen)
    (CallFunction|ForwardTracer)
    (switch Utilities|FlowControl|Switch|SwitchonE_AI_JumpState (Variables|Default|GetBoss_JumpState)
      (:NewEnumerator2
        (CallFunction|JumpEvent))
      (:NewEnumerator3
        (CallFunction|HandandClimb)))))

(event EventSetWalkSpeed
  (params (speed :type Float%20%28single-precision%29))
  (Variables|/Script/Engine.CharacterMovementComponent|SetMaxWalkSpeed (Variables|Character|GetCharacterMovement) speed))

(event OnComponentBeginOverlap(CatchPlayerCollision)
  (params (OverlappedComponent :type Primitive%20Component%20Object%20Reference) (OtherActor :type Actor%20Object%20Reference) (OtherComp :type Primitive%20Component%20Object%20Reference) (OtherBodyIndex :type Integer) (bFromSweep :type Boolean) (SweepResult :type Hit%20Result%20Structure%20%28by%20ref%29))
  (Utilities|Casting|CastToFPSMannequin OtherActor)
  (Variables|Default|SetbPlayerIsCatched true)
  (Utilities|FlowControl|Delay 5.0)
  (Variables|Default|SetbPlayerIsCatched false))

(event OnHearNoise(PawnSensingComp)
  (params (Instigator :type Pawn%20Object%20Reference) (Location :type Vector%20%28by%20ref%29 :default "0, 0, 0") (Volume :type Float%20%28single-precision%29)))

(event Custom|SR_VictorAnim
  ;[1 0 0] Attack Anim Play Server & MultiCast
  (Animation|PlayAnimMontage "/Game/AICharacter/BOOS/AM_Victory.AM_Victory" 0.8 "None"))

(event Custom|MC_PlayAttackAnim
  ;[1 0 0] Attack Anim Play Server & MultiCast
  (Animation|PlayAnimMontage "/Game/AICharacter/BOOS/AM_Attack.AM_Attack" 3.0 "None"))

(event EventPlayVictoryAnim
  ;[1 0 0] Attack Anim Play Server & MultiCast
  (CallFunction|SRVictorAnim))

(event EventPlayAttackAnim
  ;[1 0 0] Attack Anim Play Server & MultiCast
  (CallFunction|MCPlayAttackAnim))

(event EventSetSuspicious
  (params (Enable :type Boolean))
  (Variables|Default|SetbPlayerSuspect Enable))

(event EventSetForwardTracer
  (params (enabale :type Boolean))
  (Variables|Default|SetPlayerIsSeen enabale))

(event Custom|PlayTurnAnim
  (bind _returnvalue (Class|FPSAICharacter|GetHitDirection))
  (bind _mapturnanim (Variables|Default|GetMapTurnAnim))
  (bind (_value _returnvalue_2) (Utilities|Map|Find _mapturnanim _returnvalue))
  (if _returnvalue_2
    (Animation|PlayAnimMontage "/Game/AICharacter/BOOS/Anim/Shoot/AM_Turn_Boss.AM_Turn_Boss" 1.0 _value)))

(event EventSetbHit
  (params (Enable :type Boolean))
  (Variables|Default|SetbHit Enable))

(event EventGetTurnEvent
  (CallFunction|PlayTurnAnim))

(fn ConstructionScript
  (Variables|/Script/Engine.CharacterMovementComponent|SetMaxWalkSpeed (Variables|Character|GetCharacterMovement) 2.5e+02))

(fn GetEnableJumpAttack
  (return (Variables|Default|GetbAttackJump)))

(fn GetSuspicious
  (return (Variables|Default|GetbPlayerSuspect)))

(fn ForwardTracer
  (bind _returnvalue (Transformation|GetActorLocation))
  (bind (_outhit _returnvalue_2) (Collision|SphereTraceByChannel _returnvalue (+ _returnvalue (* (Transformation|GetActorForwardVector) 2e+02)) 2e+01 "TraceTypeQuery4" false (Utilities|Array|MakeArray 0) "ForDuration"))
  (bind _output_get (Variables|Default|SetWallLocation (.Location (Collision|BreakHitResult _outhit))))
  (Variables|Default|SetWall%20Noraml (.Normal (Collision|BreakHitResult _outhit)))
  (if _returnvalue_2
    (bind (_outhit_2 _returnvalue_3) (Collision|SphereTraceByChannel (+ (+ (* (.Normal (Collision|BreakHitResult _outhit)) -2e+01) _output_get) (Math|Vector|MakeVector 0.0 0.0 (Variables|Default|GetMaxJumpLenght))) (+ (* (.Normal (Collision|BreakHitResult _outhit)) -2e+01) _output_get) 2e+01 "TraceTypeQuery4" false (Utilities|Array|MakeArray 0) "ForDuration"))
    (bind _output_get_2 (Variables|Default|SetHitLedgeUp _outhit_2))
    (if _returnvalue_3
      (if (!= (.Distance (Collision|BreakHitResult _output_get_2)) 0.0)
        (bind _output_get_3 (Variables|Default|SetLedgeHeight (- (Variables|Default|GetMaxJumpLenght) (.Distance (Collision|BreakHitResult _output_get_2)))))
        (if (< _output_get_3 45.0)
          (Variables|Default|SetBoss_JumpState "NewEnumerator1")
          (elif (and (>= _output_get_3 45.0) (<= _output_get_3 85.0))
            (Variables|Default|SetBoss_JumpState "NewEnumerator2")
            (else
              (Variables|Default|SetBoss_JumpState "NewEnumerator3"))))))))

(fn GetJumpPermision
  ;[1 1 1] Jump Version_2 no more use it
  (return (Variables|Default|GetbJumpOn)))

(fn CalculateHangonLocation
  (bind _wall_noraml (Variables|Default|GetWall%20Noraml))
  (LocalVariables|SetHangOnTargetLocation (- (.impactpoint (Variables|Default|GetHitLedgeUp)) (Math|Vector|MakeVector 0.0 0.0 (+ (Components|Capsule|GetScaledCapsuleHalfHeight (Variables|Default|GetCapsuleComponent)) 2e+01))))
  (if (or (> (.x _wall_noraml) 0.0) (> (.y _wall_noraml) 0.0))
    (if (> (.x (Variables|Default|GetWall%20Noraml)) 0.0)
      (LocalVariables|SetHangOnTargetLocation (Math|Vector|MakeVector (+ (.x (LocalVariables|GetHangOnTargetLocation)) (LocalVariables|GetLedgDistance)) (.y (LocalVariables|GetHangOnTargetLocation)) (.z (LocalVariables|GetHangOnTargetLocation))))
      (else
        (LocalVariables|SetHangOnTargetLocation (Math|Vector|MakeVector (.x (LocalVariables|GetHangOnTargetLocation)) (+ (.y (LocalVariables|GetHangOnTargetLocation)) (LocalVariables|GetLedgDistance)) (.z (LocalVariables|GetHangOnTargetLocation))))))
    (elif (> (.x (Variables|Default|GetWall%20Noraml)) 0.0)
      (LocalVariables|SetHangOnTargetLocation (Math|Vector|MakeVector (- (.x (LocalVariables|GetHangOnTargetLocation)) (LocalVariables|GetLedgDistance)) (.y (LocalVariables|GetHangOnTargetLocation)) (.z (LocalVariables|GetHangOnTargetLocation))))
      (else
        (LocalVariables|SetHangOnTargetLocation (Math|Vector|MakeVector (.x (LocalVariables|GetHangOnTargetLocation)) (- (.y (LocalVariables|GetHangOnTargetLocation)) (LocalVariables|GetLedgDistance)) (.z (LocalVariables|GetHangOnTargetLocation)))))))
  (return (LocalVariables|GetHangOnTargetLocation)))

(fn Alarming
  (return (Class|FPSAICharacter|GetAlarm)))

(fn GetAlarmActor
  (return (Class|FPSAICharacter|GetAlarmInstigator)))

(fn GetbHit
  (return (Variables|Default|GetbHit)))

(fn IsObservedEnemy
  (params (ObservedActor :type Actor%20Object%20Reference))
  (bind _tags (Variables|/Script/Engine.Actor|GetTags ObservedActor))
  (bind _enemy (Variables|Default|GetEnemy))
  (bind _output (Utilities|Array|Get(acopy) _tags))
  (bind _returnvalue (Utilities|Name|Equal(Name) _output _enemy))
  (Utilities|IsValid ObservedActor
    (:Is%20Valid
      (if _returnvalue
        (bind _output_get (Variables|Default|SetPlayerIsSeen _returnvalue))
        (return _output_get)))))

(fn PlayerIsCatched
  (return (Variables|Default|GetbPlayerIsCatched)))