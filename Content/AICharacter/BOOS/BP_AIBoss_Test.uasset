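; Test boss AI character that tracks suspicion, player-seen and caught states, exposed through setters and getters.
; Each tick, forward and downward sphere traces measure ledges to set a jump state, whose handling branches are still empty.
; Overlapping the catch collision flags an FPSMannequin player as caught for five seconds.
; Server/multicast-style events play attack and victory montages, while movement and behavior-tree startup logic is disconnected.
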(event EventBeginPlay)

(event EventTick
  (params (DeltaSeconds :type Float%20%28single-precision%29))
  (CallFunction|ForwardTracer)
  (switch Utilities|FlowControl|Switch|SwitchonE_AI_JumpState (Variables|Default|GetBoss_JumpState)
    (:NewEnumerator1
      _)
    (:NewEnumerator2
      _)
    (:NewEnumerator3
      _)
    (:NewEnumerator4
      _))
  (Development|PrintString (Utilities|String|Append "Ledge Height = " (Utilities|String|ToString(Float) (.Distance (Collision|BreakHitResult (Variables|Default|GetHitLedgeUp)))))))

(event EventSetWalkSpeed
  (params (speed :type Float%20%28single-precision%29))
  (Variables|/Script/Engine.CharacterMovementComponent|SetMaxWalkSpeed (Variables|Character|GetCharacterMovement) speed))

(event OnComponentBeginOverlap(CatchPlayerCollision)
  (params (OverlappedComponent :type Primitive%20Component%20Object%20Reference) (OtherActor :type Actor%20Object%20Reference) (OtherComp :type Primitive%20Component%20Object%20Reference) (OtherBodyIndex :type Integer) (bFromSweep :type Boolean) (SweepResult :type Hit%20Result%20Structure%20%28by%20ref%29))
  (Utilities|Casting|CastToFPSMannequin OtherActor)
  (Variables|Default|SetbPlayerIsCatched true)
  (Utilities|FlowControl|Delay 5.0)
  (Variables|Default|SetbPlayerIsCatched false))

(event OnHearNoise(PawnSensingComp)
  (params (Instigator :type Pawn%20Object%20Reference) (Location :type Vector%20%28by%20ref%29 :default "0, 0, 0") (Volume :type Float%20%28single-precision%29)))

(event Custom|SR_VictorAnim
  ;[1 0 0] Attack Anim Play Server & MultiCast
  (Animation|PlayAnimMontage "/Game/AICharacter/BOOS/AM_Victory.AM_Victory" 0.8 "None"))

(event Custom|MC_PlayAttackAnim
  ;[1 0 0] Attack Anim Play Server & MultiCast
  (Animation|PlayAnimMontage "/Game/AICharacter/BOOS/AM_Attack.AM_Attack" 3.0 "None"))

(event EventPlayVictoryAnim
  ;[1 0 0] Attack Anim Play Server & MultiCast
  (CallFunction|SRVictorAnim))

(event EventPlayAttackAnim
  ;[1 0 0] Attack Anim Play Server & MultiCast
  (CallFunction|MCPlayAttackAnim))

(event EventSetSuspicious
  (params (Enable :type Boolean))
  (Variables|Default|SetbPlayerSuspect Enable))

(event EventSetForwardTracer
  (params (enabale :type Boolean))
  (Variables|Default|SetPlayerIsSeen enabale))

(fn ConstructionScript
  (Variables|/Script/Engine.CharacterMovementComponent|SetMaxWalkSpeed (Variables|Character|GetCharacterMovement) 2.5e+02))

(fn GetEnableJumpAttack
  (return (Variables|Default|GetbAttackJump)))

(fn GetSuspicious
  (return (Variables|Default|GetbPlayerSuspect)))

(fn ForwardTracer
  (bind _returnvalue (Transformation|GetActorLocation))
  (bind _returnvalue_2 (Transformation|GetActorRotation))
  (bind _returnvalue_3 (Transformation|GetActorLocation))
  (bind _returnvalue_4 (Transformation|GetActorRotation))
  (bind _returnvalue_5 (Math|Vector|GetForwardVector _returnvalue_4))
  (bind _returnvalue_6 (Math|Vector|GetForwardVector _returnvalue_2))
  (bind _returnvalue_7 (+ (.z _returnvalue) 2e+02))
  (bind _returnvalue_8 (Math|Vector|MakeVector (.x _returnvalue) (.y _returnvalue) _returnvalue_7))
  (bind _returnvalue_9 (* _returnvalue_6 7e+01))
  (bind _returnvalue_10 (+ _returnvalue_8 _returnvalue_9))
  (bind (_x _y _z) (Math|Vector|BreakVector _returnvalue_10))
  (bind (_outhit _returnvalue_11) (Collision|SphereTraceByChannel _returnvalue_3 (+ _returnvalue_3 (Math|Vector|MakeVector (* (.x _returnvalue_5) 1.5e+02) (* (.y _returnvalue_5) 1.5e+02) (.z _returnvalue_5))) 2e+01 "TraceTypeQuery4" false (Utilities|Array|MakeArray 0) "ForOneFrame"))
  (Variables|Default|SetWallLocation (.Location (Collision|BreakHitResult _outhit)))
  (Variables|Default|SetWall%20Noraml (.Normal (Collision|BreakHitResult _outhit)))
  (if _returnvalue_11
    (bind (_outhit_2 _returnvalue_12) (Collision|SphereTraceByChannel _returnvalue_10 (Math|Vector|MakeVector _x _y (- _z 2e+02)) 2e+01 "TraceTypeQuery4" false (Utilities|Array|MakeArray 0) "ForOneFrame"))
    (bind _output_get (Variables|Default|SetHitLedgeUp _outhit_2))
    (if _returnvalue_12
      (if (< (.Distance (Collision|BreakHitResult _output_get)) 6e+01)
        (Variables|Default|SetBoss_JumpState "NewEnumerator1")
        (elif (and (>= (.Distance (Collision|BreakHitResult _output_get)) 6e+01) (>= (.Distance (Collision|BreakHitResult _output_get)) 8e+01))
          (Variables|Default|SetBoss_JumpState "NewEnumerator2")
          (else
            (Variables|Default|SetBoss_JumpState "NewEnumerator3")))))))

(fn IsObservedEnemy
  (params (ObservedActor :type Actor%20Object%20Reference))
  (bind _tags (Variables|/Script/Engine.Actor|GetTags ObservedActor))
  (bind _enemy (Variables|Default|GetEnemy))
  (bind _output (Utilities|Array|Get(acopy) _tags))
  (bind _returnvalue (Utilities|Name|Equal(Name) _output _enemy))
  (Utilities|IsValid ObservedActor
    (:Is%20Valid
      (if _returnvalue
        (bind _output_get (Variables|Default|SetPlayerIsSeen _returnvalue))
        (return _output_get)))))

(fn PlayerIsCatched
  (return (Variables|Default|GetbPlayerIsCatched)))