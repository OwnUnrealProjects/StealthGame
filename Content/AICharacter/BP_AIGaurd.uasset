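; BP_AIGaurd is an AI guard character that shows its awareness state above itself.
; On BeginPlay it caches its BP_AIController.
; OnStateChanged casts the GaurdSatate widget component to WBP_GuardState and sets its text to blank, "?" or "!" for Idle, Suspisious or Alert.
; An unconnected GetGuardState call is left noted for Blueprint-driven patrolling.
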(event EventBeginPlay
  (bind _asbp_aicontroller (Utilities|Casting|CastToBP_AIController (Pawn|GetController)))
  (Variables|Default|SetOwnController _asbp_aicontroller))

(event Collision|EventActorBeginOverlap
  (params (OtherActor :type Actor%20Object%20Reference)))

(event EventTick
  (params (DeltaSeconds :type Float%20%28single-precision%29)))

(event EventOnStateChanged
  (params (NewState :type EAIState%20Enum :default "Idle"))
  (bind _aswbp_guard_state (Utilities|Casting|CastToWBP_GuardState (UserInterface|GetUserWidgetObject (Variables|Default|GetGaurdSatate))))
  (Default|UpdateText _aswbp_guard_state (Utilities|Select :Index NewState :Idle "" :Suspisious "?" :Alert "!")))

(fn ConstructionScript)