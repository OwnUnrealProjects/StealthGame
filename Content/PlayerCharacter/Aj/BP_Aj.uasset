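; BP_Aj is the player character Blueprint for Aj, defining that character's movement and feature stats.
; The construction script fills the OwnFeatures struct with Aj's values and applies its MaxSpeed to the movement component's walk speed.
; BeginPlay only calls the parent, and the crouch events are empty, with unconnected speed-switching logic and a note to move it to C++.
; The remaining event graph nodes are inactive debug prints and stubs.
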(event EventBeginPlay
  (|CallParentFunction))

(event Collision|EventActorBeginOverlap
  (params (OtherActor :type Actor%20Object%20Reference)))

(event EventTick
  (params (DeltaSeconds :type Float%20%28single-precision%29)))

(event Custom|CL_Crouch
  (params (bCrouch :type Boolean))
  ;[1 1 1] Put it in C++
  ;;[1 1 1] Set Crouch for Owner
)

(event EventCanCrouched
  (params (Enable :type Boolean))
  ;[1 1 1] Put it in C++
  ;;[1 1 1] Executed Crouch
)

(fn ConstructionScript
  (bind _output_get (Variables|Default|SetOwnFeatures (Utilities|Struct|MakeCharcterFeature 8e+02 4e+02 0.5 8e+03 7e+01 6.0 "/Game/PlayerCharacter/Aj/Aj.Aj")))
  (Variables|/Script/Engine.CharacterMovementComponent|SetMaxWalkSpeed (Variables|Character|GetCharacterMovement) (.maxspeed _output_get)))