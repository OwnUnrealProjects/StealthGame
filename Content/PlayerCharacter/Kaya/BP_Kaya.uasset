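; BP_Kaya is the Blueprint for the player character Kaya, mostly holding per-character setup and debug helpers.
; The construction script fills the OwnFeatures struct and applies its MaxSpeed to CharacterMovement's walk speed.
; BeginPlay prints the actor's name, and HeadCollision hits draw a debug arrow to the impact point.
; Crouch events are empty stubs marked for C++, with old replicated crouch-speed logic left disconnected.
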(event OnComponentHit(HeadCollision)
  (params (HitComponent :type Primitive%20Component%20Object%20Reference) (OtherActor :type Actor%20Object%20Reference) (OtherComp :type Primitive%20Component%20Object%20Reference) (NormalImpulse :type Vector :default "0, 0, 0") (Hit :type Hit%20Result%20Structure%20%28by%20ref%29))
  (Rendering|Debug|DrawDebugArrow (Transformation|GetWorldLocation (Variables|Default|GetHeadCollision)) (.ImpactPoint (Collision|BreakHitResult Hit)) 1e+01 "(R=1.000000,G=0.144519,B=0.034841,A=1.000000)" 1e+01 5.0))

(event EventBeginPlay
  (Development|PrintString (Utilities|GetDisplayName self) true true "(R=0.291683,G=1.000000,B=0.130349,A=1.000000)" 2e+01))

(event Collision|EventActorBeginOverlap
  (params (OtherActor :type Actor%20Object%20Reference)))

(event EventTick
  (params (DeltaSeconds :type Float%20%28single-precision%29)))

(event Custom|CL_Crouch
  (params (bCrouch :type Boolean))
  ;[1 1 1] Put it in C++
  ;;[1 1 1] Set Crouch for Owner
)

(event EventCanCrouched
  (params (Enable :type Boolean))
  ;[1 1 1] Put it in C++
  ;;[1 1 1] Executed Crouch
)

(fn ConstructionScript
  (bind _output_get (Variables|Default|SetOwnFeatures (Utilities|Struct|MakeCharcterFeature 6e+02 2.5e+02 0.2 1e+04 1e+01 8.0 "/Game/PlayerCharacter/Kaya/Kaya.Kaya")))
  (Variables|/Script/Engine.CharacterMovementComponent|SetMaxWalkSpeed (Variables|Character|GetCharacterMovement) (.maxspeed _output_get)))