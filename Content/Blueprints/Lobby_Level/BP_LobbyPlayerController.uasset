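; Lobby player controller that shows the lobby UI, relays menu input and records the player's data and ready state.
; On BeginPlay, only the local controller creates WBP_Lobby and caches the lobby GameState, which Tick polls to update MaxPlayer.
; Ready, Previous and Next inputs fire key-press dispatchers for widget binding.
; SetPlayerData writes the chosen data to FPSPlayerState and sets ReadyToStart.
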(event Custom|SetPlayerData
  (params (NewParam :type Player%20Data%20Structure))
  ;[1 1 1] Set Pawn Data to PlayerState
  (bind _asfpsplayer_state (Utilities|Casting|CastToFPSPlayerState (Variables|GetPlayerState)))
  (Class|FPSPlayerState|SetOwnerPlayerData _asfpsplayer_state NewParam)
  (Variables|Default|SetbReadyToStart true))

(event EventBeginPlay
  ;[1 1 1] Create Widget Only for Localy Controller
  (if (Pawn|IsLocalController)
    (bind _returnvalue (UserInterface|CreateWidget "/Game/UI/WBP_Lobby.WBP_Lobby_C"))
    (UserInterface|Viewport|AddtoViewport _returnvalue 0)
    (bind _asbp_lobby_game_state (Utilities|Casting|CastToBP_LobbyGameState (Game|GetGameState)))
    (Variables|Default|SetLobbyGameState _asbp_lobby_game_state)
    (bind _output_get (Variables|Default|SetLobbyWidget _returnvalue))))

(event EventTick
  (params (DeltaSeconds :type Float%20%28single-precision%29))
  (bind _lobbygamestate (Variables|Default|GetLobbyGameState))
  (if (Utilities|IsValid _lobbygamestate)
    (Variables|Default|SetMaxPlayer (Variables|/Game/Blueprints/Lobby_Level/BP_LobbyGameState.BP_LobbyGameState_C|GetPlayerNumber _lobbygamestate))))

(event Input|ActionEvents|InputActionReady
  (params (Key :type Key%20Structure))
  ;[1 1 1] Input Bind To Widget
  (:Pressed
    (Default|CallDispatcherKeyPressEnter Key)))

(event Input|ActionEvents|InputActionPrevious
  (params (Key :type Key%20Structure))
  ;[1 1 1] Input Bind To Widget
  (:Pressed
    (Default|CallDispatcherKeyPressLeft Key)))

(event Input|ActionEvents|InputActionNext
  (params (Key :type Key%20Structure))
  ;[1 1 1] Input Bind To Widget
  (:Pressed
    (Default|CallDispatcherKeyPressRight Key)))

(fn ConstructionScript)