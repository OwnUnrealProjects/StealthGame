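; BP_LobbyGameMode is the lobby level's game mode, which caches the host's lobby player controller.
; On BeginPlay it casts player controller 0 to BP_LobbyPlayerController and stores it as ServerPlayerController if it is local.
; Tick is empty, and the match-start logic is disconnected: a one-shot level open on the widget's StartGame flag, plus a servertravel and StartSession variant.
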(event EventBeginPlay
  (bind _returnvalue (Game|GetPlayerController 0))
  (bind _asbp_lobby_player_controller (Utilities|Casting|CastToBP_LobbyPlayerController _returnvalue))
  (if (Pawn|IsLocalController _returnvalue)
    (Variables|Default|SetServerPlayerController _asbp_lobby_player_controller)))

(event EventTick
  (params (DeltaSeconds :type Float%20%28single-precision%29)))

(fn ConstructionScript)