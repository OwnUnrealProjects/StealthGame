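; Player controller Blueprint for an FPS game that shows the game-over screen when a mission ends.
; OnMissionCompleted creates a WBP_GameOver widget with the mission success flag and adds it to the viewport.
; On BeginPlay it prints, as debug output, the player name from the TestPlayerState held in FPSInGameInstance, or a notice if that state is invalid.
; Some leftover PlayerState cast and delay nodes are disconnected.
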(event EventBeginPlay
  (bind _asfpsin_game_instance (Utilities|Casting|CastToFPSInGameInstance (Game|GetGameInstance)))
  (Utilities|IsValid (Variables|/Script/FPSGame.FPSInGameInstance|GetTestPlayerState _asfpsin_game_instance)
    (:Is%20Valid
      (Development|PrintString (PlayerState|GetPlayerName (Variables|/Script/FPSGame.FPSInGameInstance|GetTestPlayerState _asfpsin_game_instance)) true true "(R=0.130723,G=1.000000,B=0.333974,A=1.000000)" 1e+01))
    (:Is%20Not%20Valid
      (Development|PrintString "TestPlayerState is NULL" true true "(R=0.130723,G=1.000000,B=0.333974,A=1.000000)" 1e+01))))

(event EventOnMissionCompleted
  (params (bMissionSuccess :type Boolean))
  (bind _returnvalue (UserInterface|CreateWidget "/Game/UI/WBP_GameOver.WBP_GameOver_C" 0 bMissionSuccess))
  (UserInterface|Viewport|AddtoViewport _returnvalue 0))

(fn ConstructionScript)