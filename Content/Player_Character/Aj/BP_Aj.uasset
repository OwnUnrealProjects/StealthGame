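; Player character Blueprint for Aj, mainly configuring that character's feature values.
; The construction script fills the OwnFeatures struct and applies its MaxSpeed to the movement component's walk speed.
; Crouch events for server and owning client are empty stubs, with their speed-switching logic left disconnected and noted for C++.
; Remaining event graph logic is empty events and unreachable debug prints.
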(event EventBeginPlay)

(event Collision|EventActorBeginOverlap
  (params (OtherActor :type Actor%20Object%20Reference)))

(event EventTick
  (params (DeltaSeconds :type Float%20%28single-precision%29)))

(event Custom|SR_Crouch
  (params (bCrouch :type Boolean))
  ;[1 1 1] Put it in C++
  ;;[1 1 1] Set Crouch On Server
)

(event Custom|CL_Crouch
  (params (bCrouch :type Boolean))
  ;[1 1 1] Put it in C++
  ;;[1 1 1] Set Crouch for Owner
)

(event EventCanCrouched
  (params (Enable :type Boolean))
  ;[1 1 1] Put it in C++
  ;;[1 1 1] Executed Crouch
)

(fn ConstructionScript
  (bind _output_get (Variables|Default|SetOwnFeatures (Utilities|Struct|MakeCharcterFeature 6e+02 4e+02 0.5 8e+03 7.0 "/Game/Player_Character/Aj/Aj.Aj")))
  (Variables|/Script/Engine.CharacterMovementComponent|SetMaxWalkSpeed (Variables|Character|GetCharacterMovement) (.maxspeed _output_get)))