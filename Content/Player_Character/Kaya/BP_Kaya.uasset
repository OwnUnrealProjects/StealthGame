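; Player character Blueprint for Kaya that sets up her movement stats and holds leftover crouch logic.
; The construction script fills the OwnFeatures struct, caches max and crouch speeds from it, and applies walk speed.
; Server and owner crouch events toggle walk speed using a hard-coded crouch value rather than the cached one.
; CanCrouched is empty and marked for C++, with its crouch calls disconnected, as are the debug prints.
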(event EventBeginPlay)

(event Collision|EventActorBeginOverlap
  (params (OtherActor :type Actor%20Object%20Reference)))

(event EventTick
  (params (DeltaSeconds :type Float%20%28single-precision%29)))

(event Custom|SR_Crouch
  (params (bCrouch :type Boolean))
  (bind _charactermovement (Variables|Character|GetCharacterMovement))
  ;[1 1 1] Put it in C++
  ;;[1 1 1] Set Crouch On Server
  (bind _output_get (Variables|Default|SetbCrouch bCrouch))
  (if _output_get
    (Variables|/Script/Engine.CharacterMovementComponent|SetMaxWalkSpeed _charactermovement 2e+02)
    (else
      (Variables|/Script/Engine.CharacterMovementComponent|SetMaxWalkSpeed _charactermovement (Variables|Default|GetDefaultMaxSpeed)))))

(event Custom|CL_Crouch
  (params (bCrouch :type Boolean))
  (bind _charactermovement (Variables|Character|GetCharacterMovement))
  ;[1 1 1] Put it in C++
  ;;[1 1 1] Set Crouch for Owner
  (bind _output_get (Variables|Default|SetbCrouch bCrouch))
  (if _output_get
    (Variables|/Script/Engine.CharacterMovementComponent|SetMaxWalkSpeed _charactermovement 2e+02)
    (else
      (Variables|/Script/Engine.CharacterMovementComponent|SetMaxWalkSpeed _charactermovement (Variables|Default|GetDefaultMaxSpeed)))))

(event EventCanCrouched
  (params (Enable :type Boolean))
  ;[1 1 1] Put it in C++
  ;;[1 1 1] Executed Crouch
)

(fn ConstructionScript
  (bind _output_get (Variables|Default|SetOwnFeatures (Utilities|Struct|MakeCharcterFeature 4e+02 2e+02 5.0 0.0 0.0 "/Game/Player_Character/Kaya/Kaya.Kaya")))
  (bind _output_get_2 (Variables|Default|SetDefaultMaxSpeed (.maxspeed _output_get)))
  (Variables|/Script/Engine.CharacterMovementComponent|SetMaxWalkSpeed (Variables|Character|GetCharacterMovement) _output_get_2)
  (Variables|Default|SetDefaultCrouchSpeed (.crouchspeed _output_get)))